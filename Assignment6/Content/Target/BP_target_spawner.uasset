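; Target spawner Blueprint that keeps spawning Bp_Target actors inside a box volume sized from BoxExtent in the construction script.
; BeginPlay starts a looping timer and also triggers a few initial spawns.
; Each timer tick counts all Bp_Target actors in the world and, under a cap, spawns one at a random point in SpawnArea.
; New targets rotate toward the player camera, with pitch offset by 90 degrees.
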(event Custom|Spawn_Target
  (bind _spawn_area (Variables|Default|GetSpawn_Area))
  (bind _outactors (Actor|GetAllActorsOfClass "/Game/Target/Bp_Target.Bp_Target_C"))
  (if (<= (Utilities|Array|Length _outactors) 10)
    (bind _output_get (Variables|Default|SetSpawnLoation (Math|Random|RandomPointinBoundingBox (Transformation|GetWorldLocation _spawn_area) (Components|Box|GetScaledBoxExtent _spawn_area))))
    (Game|SpawnActorfromClass "/Game/Target/Bp_Target.Bp_Target_C" (Math|Transform|MakeTransform _output_get (Math|Rotator|MakeRotator (.roll (Math|Rotator|FindLookatRotation _output_get (Transformation|GetWorldLocation (Variables|/Script/Engine.PlayerCameraManager|GetTransformComponent (Game|GetPlayerCameraManager 0))))) (- (.pitch (Math|Rotator|FindLookatRotation _output_get (Transformation|GetWorldLocation (Variables|/Script/Engine.PlayerCameraManager|GetTransformComponent (Game|GetPlayerCameraManager 0))))) 9e+01) (.yaw (Math|Rotator|FindLookatRotation _output_get (Transformation|GetWorldLocation (Variables|/Script/Engine.PlayerCameraManager|GetTransformComponent (Game|GetPlayerCameraManager 0)))))) "1.000000,1.000000,1.000000") "AdjustIfPossibleButAlwaysSpawn" "MultiplyWithRoot" 0 0)))

(event EventBeginPlay
  (Utilities|Time|SetTimerbyEvent (delegate Custom|Spawn_Target) 1.0 true)
  ;[1 1 1] ?
  (for _index (range 0 2)
    (CallFunction|SpawnTarget)))

(fn ConstructionScript
  (Components|Box|SetBoxExtent (Variables|Default|GetSpawn_Area) (Variables|Default|GetBox%20Extent) true))