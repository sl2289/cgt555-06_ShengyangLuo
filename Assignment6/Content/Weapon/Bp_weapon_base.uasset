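; Base weapon Blueprint that handles magazine ammo, firing and timed reloading, leaving Weapontrace as an empty event.
; Fireweapon spends a round, spawns muzzle emitter and sound at the Arrow, then calls Weapontrace, or reloads when empty.
; Both reload events show a WB_ReloadBar animation and refill after Reloadtime, with no guard against firing meanwhile.
; A getter exposes the weapon's FOV multiplier.
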(event Custom|ReloadWeapon
  (bind _returnvalue (UserInterface|CreateWidget "/Game/Weapon/WB_ReloadBar.WB_ReloadBar_C"))
  (Default|ReloadAnimation _returnvalue (Variables|Ammo|GetReloadtime))
  (UserInterface|Viewport|AddtoViewport _returnvalue 0)
  (Utilities|FlowControl|Delay (Variables|Ammo|GetReloadtime))
  (Variables|Ammo|SetAmmo (Variables|Ammo|GetMaxmagezineAmmo)))

(event Custom|Weapontrace)

(event EventBeginPlay
  (Variables|Ammo|SetAmmo (Variables|Ammo|GetMaxmagezineAmmo)))

(event EventReload
  (bind _returnvalue (UserInterface|CreateWidget "/Game/Weapon/WB_ReloadBar.WB_ReloadBar_C"))
  (Default|ReloadAnimation _returnvalue (Variables|Ammo|GetReloadtime))
  (UserInterface|Viewport|AddtoViewport _returnvalue 0)
  (Utilities|FlowControl|Delay (Variables|Ammo|GetReloadtime))
  (Variables|Ammo|SetAmmo (Variables|Ammo|GetMaxmagezineAmmo)))

(event EventFireweapon
  (if (<= (Variables|Ammo|GetAmmo) 0)
    (CallFunction|ReloadWeapon)
    (else
      (Variables|Ammo|SetAmmo (- (Variables|Ammo|GetAmmo) 1))
      (CallFunction|WeaponFireEffects)
      (CallFunction|Weapontrace))))

(fn ConstructionScript)

(fn WeaponFireEffects
  (bind _arrow (Variables|Default|GetArrow))
  (bind _returnvalue (Transformation|GetWorldTransform _arrow))
  (Effects|SpawnEmitteratLocation (Variables|WeaponFireEffects|GetWeaponFireEmitter) (.location _returnvalue) (.rotation _returnvalue) (Variables|WeaponFireEffects|GetWeaponFireEmitterScale))
  (Audio|SpawnSoundatLocation (Variables|WeaponFireEffects|GetWeaponFireSounds) (.location _returnvalue) "0, 0, 0" 1.0 1.0 0.0 0 0)
  (return))

(fn GetFOVMultiplayer
  (return (Variables|Default|GetFOVmultiler)))